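; BP_CombatInput is a possessable test pawn that switches the combat input mapping on and off with possession.
; On possession by a BP_PlayerController it moves to that controller's transform and adds IMC_Combat through the controller's Enhanced Input local player subsystem.
; On unpossession it removes the context, so the mapping follows possession, and it binds no input actions itself.
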(event `self.ReceivePossessed`
  (params (NewController :type "Controller Object Reference"))
  (bind _asbp_player_controller (cast `/Game/Testing/Input/BP_PlayerController` NewController))
  (`self.K2_SetActorTransform` (`self.GetTransform` _asbp_player_controller))
  (bind _returnvalue (pcsubsystem `EnhancedInputLocalPlayerSubsystem` _asbp_player_controller))
  (`/Engine/EditorBlueprintResources/StandardMacros.IsValid` _returnvalue
    (:`Is Valid`
      (message `EnhancedInputSubsystemInterface.AddMappingContext` _returnvalue "/Game/Testing/Input/Gameplay/IMC_Combat.IMC_Combat" 0 (struct)))))

(event `self.ReceiveUnpossessed`
  (params (OldController :type "Controller Object Reference"))
  (bind _asbp_player_controller (cast `/Game/Testing/Input/BP_PlayerController` OldController))
  (bind _returnvalue (pcsubsystem `EnhancedInputLocalPlayerSubsystem` _asbp_player_controller))
  (`/Engine/EditorBlueprintResources/StandardMacros.IsValid` _returnvalue
    (:`Is Valid`
      (`EnhancedInputSubsystemInterface.RemoveMappingContext` _returnvalue "/Game/Testing/Input/Gameplay/IMC_Combat.IMC_Combat" (struct)))))

(fn `UserConstructionScript`)