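; BP_DjinniBase is the base Blueprint for a Djinni, holding a name, element, state and stat block tied to an owning Adept.
; SetState stores the new state and applies its stat effect: Set subtracts the Djinni's BaseStats from the owner's, while Standby adds them.
; The owner's BaseStats are modified in place field by field, with no check of the previous state.
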(fn `Add Base Stats`
  (bind (_basestats_hp _basestats_pp _basestats_attack _basestats_defense _basestats_agility _basestats_luck) (break `UnitStats` (`self.BaseStats`)))
  (bind (_basestats_hp_2 _basestats_pp_2 _basestats_attack_2 _basestats_defense_2 _basestats_agility_2 _basestats_luck_2) (break `UnitStats` (`Adept.BaseStats` (`self.OwningAdept`))))
  (set `Adept.BaseStats` (make `UnitStats` (+ _basestats_hp_2 _basestats_hp) (+ _basestats_pp_2 _basestats_pp) (+ _basestats_attack_2 _basestats_attack) (+ _basestats_defense_2 _basestats_defense) (+ _basestats_agility_2 _basestats_agility) (+ _basestats_luck_2 _basestats_luck)) (`self.OwningAdept`)))

(fn `Get Element`
  (returns (Element :type "EElementalType Enum"))
  (return (`self.Element`)))

(fn `Get Name`
  (returns (Name :type String))
  (return (`self.Name`)))

(fn `Set State`
  (params (State :type "EDjinniState Enum" :default "Set"))
  (bind _output_get (set `self.State` State))
  (switch `EDjinniState` _output_get
    (:`Set`
      (`self.Subtract Base Stats`))
    (:`Standby`
      (`self.Add Base Stats`))))

(fn `Subtract Base Stats`
  (bind (_basestats_hp _basestats_pp _basestats_attack _basestats_defense _basestats_agility _basestats_luck) (break `UnitStats` (`self.BaseStats`)))
  (bind (_basestats_hp_2 _basestats_pp_2 _basestats_attack_2 _basestats_defense_2 _basestats_agility_2 _basestats_luck_2) (break `UnitStats` (`Adept.BaseStats` (`self.OwningAdept`))))
  (set `Adept.BaseStats` (make `UnitStats` (- _basestats_hp_2 _basestats_hp) (- _basestats_pp_2 _basestats_pp) (- _basestats_attack_2 _basestats_attack) (- _basestats_defense_2 _basestats_defense) (- _basestats_agility_2 _basestats_agility) (- _basestats_luck_2 _basestats_luck)) (`self.OwningAdept`)))

(fn `UserConstructionScript`)