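; BP_PsynergyBase is the base Blueprint for Psynergy abilities, holding display and targeting data such as icon, name, cost, element, target type and range.
; On BeginPlay it caches the CombatTargeting object from the custom GameInstance.
; Its ally and enemy targeting functions pass the unit and target count to CombatTargeting and begin targeting that team.
; A getter returns the ability's data in one call.
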(event `self.ReceiveBeginPlay`
  (bind _ascustom_game_instance (cast `CustomGameInstance` (`GameplayStatics.GetGameInstance`)))
  (set `self.Combat Targeting` (`CustomGameInstance.GetCombatTargeting` _ascustom_game_instance)))

(fn `Get Initializers`
  (returns (`Psynergy Icon` :type "Texture2D Object Reference") (Name :type String) (Cost :type Integer) (Element :type "EElementalType Enum") (`Target Type` :type "ETargetType Enum") (Range :type Integer))
  (return (`self.Icon`) (`self.Name`) (`self.Cost`) (`self.Element`) (`self.TargetType`) (`self.AmountOfTargets`)))

(fn `TargetAllyTeam`
  (params (Unit :type "Unit Object Reference"))
  (bind _output_get (set `CombatTargeting.CurrentUnit` Unit (`self.Combat Targeting`)))
  (set `CombatTargeting.MinorTargetAmount` (`self.AmountOfTargets`) (`self.Combat Targeting`))
  (`CombatTargeting.BeginTargeting` (`self.Combat Targeting`) _output_get "Ally"))

(fn `TargetEnemyTeam`
  (params (Unit :type "Unit Object Reference"))
  (bind _output_get (set `CombatTargeting.CurrentUnit` Unit (`self.Combat Targeting`)))
  (set `CombatTargeting.MinorTargetAmount` (`self.AmountOfTargets`) (`self.Combat Targeting`))
  (`CombatTargeting.BeginTargeting` (`self.Combat Targeting`) _output_get "Enemy"))

(fn `UserConstructionScript`)